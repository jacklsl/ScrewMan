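; ScrewMan is a Paper2D flipbook character that runs, jumps, double-jumps and slides, driven by mouse input.
; Left click starts a jump or upgrades it to a double jump, restarting the timer; holding right click sets the slide state, which blocks new jumps.
; Tick offsets height from the starting Z using float curves over a one-second jump, otherwise switching between run and slide flipbooks.
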(event `self.ReceiveBeginPlay`
  (bind (_returnvalue_x _returnvalue_y _returnvalue_z) (`KismetMathLibrary.BreakVector` (`self.K2_GetActorLocation`)))
  (set `self.OrginZ` _returnvalue_z))

(event `self.ReceiveTick`
  (params (DeltaSeconds :type "Float (single-precision)"))
  (bind (_returnvalue_x _returnvalue_y) (`KismetMathLibrary.BreakVector` (`self.K2_GetActorLocation`)))
  (bind _paperflipbook (`self.PaperFlipbook`))
  (if (`self.isOneJump`)
    (bind _output_get (set `self.MouseDurationTime` (- (`KismetSystemLibrary.GetGameTimeInSeconds`) (`self.MouseClickTime`))))
    (`self.K2_SetActorLocation` (`KismetMathLibrary.MakeVector` _returnvalue_x _returnvalue_y (+ (`self.OrginZ`) (`CurveFloat.GetFloatValue` (select `bool` (`self.isTwoJump`) :`false` (`self.OneJumpCurve`) :`true` (`self.TwoJumpCurve`)) _output_get))))
    (if (>= (`self.MouseDurationTime`) 1.0)
      (set `self.isOneJump` false)
      (set `self.isTwoJump` false)
      (`PaperFlipbookComponent.SetFlipbook` _paperflipbook "/Game/FlipBooks/Run.Run" :!label _label)
      (`PaperFlipbookComponent.SetLooping` _paperflipbook true)
      (`PaperFlipbookComponent.Play` _paperflipbook))
    (elif (`self.isSlide`)
      (`PaperFlipbookComponent.SetFlipbook` (`self.PaperFlipbook`) "/Game/FlipBooks/Slide.Slide")
      (else
        (goto _label)))))

(event `Key|LeftMouseButton`
  (bind _paperflipbook (`self.PaperFlipbook`))
  (:`Pressed`
    (if (`self.isSlide`)
      _
      (elif (not (`self.isTwoJump`))
        (if (`self.isOneJump`)
          (set `self.isTwoJump` true)
          (`PaperFlipbookComponent.SetFlipbook` _paperflipbook "/Game/FlipBooks/twojump.twojump")
          (`PaperFlipbookComponent.SetLooping` _paperflipbook false)
          (else
            (set `self.isOneJump` true)
            (`PaperFlipbookComponent.SetFlipbook` (`self.PaperFlipbook`) "/Game/FlipBooks/onejump_Flipbook.onejump_Flipbook")))
        (set `self.MouseClickTime` (`KismetSystemLibrary.GetGameTimeInSeconds`))))))

(event `Key|RightMouseButton`
  (:`Pressed`
    (set `self.isSlide` true))
  (:`Released`
    (set `self.isSlide` false)))

(fn `UserConstructionScript`)